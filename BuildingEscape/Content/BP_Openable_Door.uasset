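; BP_Openable_Door is a door actor that swings open and closed on requests from its OpenDoor component.
; The DoorOpen timeline plays forward to open and reverses to close, scaling the component's open angle into a yaw offset combined with the rotation cached at BeginPlay.
; A Sound Timing event track plays the Doorlock sound at the actor's location only while the timeline runs backward, during closing.
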(event `self.ReceiveBeginPlay`
  (set `self.StartRotation` (`self.K2_GetActorRotation`)))

(event `self.OpenDoor.OnOpenRequest`
  (bind (_direction _openinpercent) (`Timeline|DoorOpen` :!label _label)
    (:`Update`
      (`self.K2_SetActorRotation` (`KismetMathLibrary.ComposeRotators` (`self.StartRotation`) (`KismetMathLibrary.MakeRotator` 0.0 0.0 (* _openinpercent (`OpenDoor.GetOpenAngleInDegree` (`self.OpenDoor`)))))))
    (:`SoundTiming`
      (if (`|EnumEquality` _direction "Backward")
        (`GameplayStatics.PlaySoundAtLocation` "/Game/door-lock.door-lock" (`self.K2_GetActorLocation`) (struct) 1.0 1.0 0.0 null null null)))))

(event `self.OpenDoor.OnCloseRequest`
  (goto _label :!via `Reverse`))

(fn `UserConstructionScript`)